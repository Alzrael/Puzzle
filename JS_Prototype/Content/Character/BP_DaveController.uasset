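; Player controller for Dave that drives click-to-move navigation and cursor-based interaction.
; Holding left click runs a looping timer through a gate, tracing the cursor to the world, flattening the hit to character height and calling SimpleMoveToLocation, repeated on release.
; Clicks too near the character become a tiny step toward the point to force rotation.
; Lock On sends InteractMessage to I_Interactables actors under the cursor; other action sections are empty.
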(event Custom|UpdateCursorPositionInWorld
  (bind _self self)
  (bind (_worldlocation _worlddirection) (Game|Player|ConvertMouseLocationToWorldSpace _self))
  ;[1 1 1 0.211] Input Action Left Click
  (Utilities|FlowControl|Gate true
    (:Exit
      (bind (_outhit _returnvalue) (Collision|LineTraceByChannel _worldlocation (+ _worldlocation (* _worlddirection (Variables|Default|GetFloorTraceDistance))) "TraceTypeQuery5" false 0 "None"))
      (if _returnvalue
        (Variables|Default|SetLastInputLocation (CallFunction|SetZtoCharacterCurrent (.Location (Collision|BreakHitResult _outhit))))
        (Utilities|MinClickDistanceCheck
          (:True
            (AI|Navigation|SimpleMovetoLocation self (Variables|Default|GetLastInputLocation)))
          (:False
            (AI|Navigation|SimpleMovetoLocation self (CallFunction|GetMinimumDistancetoForceRotation))))))))

(event EventBeginPlay
  ;[1 0.7481 0.778] Begin play
  (Variables|Default|SetbShowMouseCursor true)
  (bind _character (Class|ICharacterInterface|GetNewCharacterReference(Message) (Pawn|GetControlledPawn) self))
  (Variables|Default|SetPlayerCharacter _character))

(event Input|ActionEvents|InputActionApperate
  (params (Key :type Key%20Structure))
  ;[1 1 1 0.211] Input Action Apperate
)

(event Input|ActionEvents|InputActionLeftClick
  (params (Key :type Key%20Structure))
  (bind _self self)
  (bind (_worldlocation _worlddirection) (Game|Player|ConvertMouseLocationToWorldSpace _self))
  ;[1 1 1 0.211] Input Action Left Click
  (:Pressed
    (bind _returnvalue (Utilities|Time|SetTimerbyEvent (EventDispatchers|CreateEvent :!event Custom|UpdateCursorPositionInWorld) (Variables|Default|GetCursorLocationCheckTime) true))
    (Variables|Default|SetCursorWorldHandle _returnvalue)
    (Utilities|FlowControl|Gate true) ; enters at Open
  )
  (:Released
    (Utilities|FlowControl|Sequence
      (:then_0
        (Utilities|Time|ClearandInvalidateTimerbyHandle (Variables|Default|GetCursorWorldHandle))
        (Utilities|FlowControl|Gate true) ; enters at Close
      )
      (:then_1
        (Utilities|MinClickDistanceCheck
          (:True
            (AI|Navigation|SimpleMovetoLocation self (Variables|Default|GetLastInputLocation)))
          (:False
            (AI|Navigation|SimpleMovetoLocation self (CallFunction|GetMinimumDistancetoForceRotation))))))))

(event Input|ActionEvents|InputActionMeleeAttack
  (params (Key :type Key%20Structure))
  ;[1 1 1 0.211] Input Action Melee Attack
)

(event Input|ActionEvents|InputActionLockOn
  (params (Key :type Key%20Structure))
  (bind _hitresult (Game|Player|GetHitResultUnderCursorbyChannel "TraceTypeQuery1" true))
  ;[1 1 1 0.211] Input Action Lock on
  (:Pressed
    (Utilities|IsValid (.hitactor _hitresult)
      (:Is%20Valid
        (if (Utilities|DoesObjectImplementInterface (.hitactor _hitresult) "/Game/Interfaces/I_Interactables.I_Interactables_C")
          (Class|IInteractables|Interact(Message) (.hitactor _hitresult)))))))

(event Input|ActionEvents|InputActionUseHealthPotion
  (params (Key :type Key%20Structure))
  ;[1 1 1 0.211] Input Action Potion Use
)

(event Input|ActionEvents|InputActionUseManaPotion
  (params (Key :type Key%20Structure))
  ;[1 1 1 0.211] Input Action Potion Use
)

(event Input|ActionEvents|InputActionWeaponSelectSlot01
  (params (Key :type Key%20Structure))
  ;[1 1 1 0.211] Input Action Weapon Slot Selection
)

(event Input|ActionEvents|InputActionWeaponSelectSlot02
  (params (Key :type Key%20Structure))
  ;[1 1 1 0.211] Input Action Weapon Slot Selection
)

(event Input|ActionEvents|InputActionWeaponSelectSlot03
  (params (Key :type Key%20Structure))
  ;[1 1 1 0.211] Input Action Weapon Slot Selection
)

(event Input|ActionEvents|InputActionWeaponSelectSlot04
  (params (Key :type Key%20Structure))
  ;[1 1 1 0.211] Input Action Weapon Slot Selection
)

(fn ConstructionScript)

(fn GetMinimumDistancetoForceRotation
  (bind _playercharacter (Variables|Default|GetPlayerCharacter))
  (bind _returnvalue (Transformation|GetActorLocation _playercharacter))
  (return (+ _returnvalue (* (Math|Vector|GetUnitDirection(Vector) _returnvalue (Variables|Default|GetLastInputLocation)) 5))))

(fn SetZtoCharacterCurrent
  (params (LocationInput :type Vector))
  (return (Math|Conversions|ToVector(Vector2D) (Math|Conversions|ToVector2D(Vector) LocationInput) (.z (Transformation|GetActorLocation (Variables|Default|GetPlayerCharacter))))))

(fn GetNewCharacterReference
  (params (Controller :type BP%20Dave%20Controller%20Object%20Reference))
  (return 0))