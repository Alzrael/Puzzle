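; Movable pillar actor that slides back and forth along the world Y axis in response to earth interactions.
; The InteractEarth event uses a FlipFlop to alternate between two timelines, one moving by positive Offset and the other by negative.
; Timeline updates serve only as a tick, each using VInterpTo toward a target relative to the current location, so travel depends on timeline length rather than a fixed endpoint.
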(event EventInteractEarth
  (bind _returnvalue (Transformation|GetActorLocation))
  (bind _returnvalue_2 (Transformation|GetActorLocation))
  (bind (_x _y _z) (Math|Vector|BreakVector _returnvalue))
  (bind (_x_2 _y_2 _z_2) (Math|Vector|BreakVector _returnvalue_2))
  (Utilities|FlowControl|FlipFlop
    (:A
      (Timeline|Timeline_0 PlayFromStart
        (:Update
          (Transformation|SetActorLocation (Math|Interpolation|VInterpTo _returnvalue (Math|Vector|MakeVector _x (+ _y (Variables|Default|GetOffset)) _z) (Utilities|Time|GetWorldDeltaSeconds) 0.5) false false))))
    (:B
      (Timeline|Move PlayFromStart
        (:Update
          (Transformation|SetActorLocation (Math|Interpolation|VInterpTo _returnvalue_2 (Math|Vector|MakeVector _x_2 (+ _y_2 (* (Variables|Default|GetOffset) -1.0)) _z_2) (Utilities|Time|GetWorldDeltaSeconds) 0.5) false false))))))

(fn ConstructionScript)