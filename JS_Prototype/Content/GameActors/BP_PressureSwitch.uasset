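; BP_PressureSwitch is a pressure switch actor that messages a linked InteractableItem when an overlap with it ends.
; On BeginPlay, a Heavy switch sets its Box collision to ignore the Pawn channel, so pawns cannot trigger it.
; End overlap calls InteractMessage on InteractableItem, while this Blueprint's begin overlap and Tick events are disabled placeholders.
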(event EventBeginPlay
  (|CallParentFunction)
  (if (Variables|Default|GetHeavy)
    (Collision|SetCollisionResponsetoChannel (Variables|Default|GetBox) "ECC_Pawn" "ECR_Ignore")))

(event Collision|EventActorBeginOverlap
  (params (OtherActor :type Actor%20Object%20Reference))
  (|CallParentFunction OtherActor) ; This node is disabled and will not be called.\nDrag off pins to build functionality.
)

(event EventTick
  (params (DeltaSeconds :type Float%20%28single-precision%29))
  (|CallParentFunction DeltaSeconds) ; This node is disabled and will not be called.\nDrag off pins to build functionality.
)

(event Collision|EventActorEndOverlap
  (params (OtherActor :type Actor%20Object%20Reference))
  (Class|IInteractables|Interact(Message) (Variables|Default|GetInteractableItem)))

(fn ConstructionScript
  (|CallParentFunction))