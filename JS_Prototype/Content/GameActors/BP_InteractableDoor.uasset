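; BP_InteractableDoor is a door actor that swings open or closed when it receives the Interact event.
; Interact passes the inverse of the Open flag to SwitchDoorState, then stores that new value.
; SwitchDoorState adds a quarter-turn world yaw to the root component in a direction set by the state, so the door snaps instantly and relies on alternating calls to stay aligned.
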(event EventInteract
  (CallFunction|SwitchDoorState (not (Variables|Default|GetOpen)))
  (Variables|Default|SetOpen (not (Variables|Default|GetOpen))))

(fn ConstructionScript)

(fn SwitchDoorState
  (params (NewState :type Boolean))
  (if NewState
    (LocalVariables|SetNewRotation -9e+01)
    (else
      (LocalVariables|SetNewRotation 9e+01)))
  (Transformation|AddWorldRotation (Variables|Default|GetDefaultSceneRoot) (Math|Rotator|MakeRotator 0.0 0.0 (LocalVariables|GetNewRotation)) false false))