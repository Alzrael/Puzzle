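; BP_InteractablePillar is an interactable pillar whose cylinder travels back and forth along a spline path.
; BeginPlay creates a paused looping timer for MoveAlongSpline, and each Interact alternately resumes or pauses it through a FlipFlop.
; Each timer tick steps the distance by Speed and moves the cylinder with a sweep, reversing direction at either spline end or on a blocking hit.
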(event EventInteract
  (bind _movealongsplinehandle (Variables|Default|GetMoveAlongSplineHandle))
  (Utilities|FlowControl|FlipFlop
    (:A
      (Utilities|Time|UnpauseTimerbyHandle _movealongsplinehandle))
    (:B
      (Utilities|Time|PauseTimerbyHandle _movealongsplinehandle))))

(event EventBeginPlay
  (bind _returnvalue (Utilities|Time|SetTimerbyFunctionName 0 "MoveAlongSpline" 0.01 true))
  (bind _output_get (Variables|Default|SetMoveAlongSplineHandle _returnvalue))
  (Utilities|Time|PauseTimerbyHandle _output_get))

(fn ConstructionScript
  (|CallParentFunction))

(fn MoveAlongSpline
  (bind _speed (Variables|Default|GetSpeed))
  (if (Variables|Default|GetForward)
    (Variables|Default|SetDistance (+ (Variables|Default|GetDistance) _speed))
    (else
      (Variables|Default|SetDistance (- (Variables|Default|GetDistance) _speed))))
  (bind _sweephitresult (Transformation|SetRelativeLocation (Variables|Default|GetCylinder) (Spline|GetLocationatDistanceAlongSpline (Variables|Default|GetPath) (Variables|Default|GetDistance) "Local") true false))
  (if (.bBlockingHit (Collision|BreakHitResult _sweephitresult))
    (Variables|Default|SetForward (not (Variables|Default|GetForward)))
    (elif (>= (Variables|Default|GetDistance) (Spline|GetSplineLength (Variables|Default|GetPath)))
      (Variables|Default|SetForward false)
      (elif (<= (Variables|Default|GetDistance) 0.0)
        (Variables|Default|SetForward true)))))