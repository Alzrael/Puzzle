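; BP_InteractableBox is an interactable box that toggles between active and inactive, with fire interaction making that toggle its last.
; Both interaction events share one toggle path, blocked once Destroyed is set.
; TriggerActive ties the cube's visibility, physics simulation and actor collision to Active.
; It also teleports the cube 500 units up when inactive and down when active, keeping it clear of movement.
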(event EventInteract
  (if (not (Variables|Default|GetDestroyed))
    (Variables|Default|SetActive (not (Variables|Default|GetActive)))
    (CallFunction|TriggerActive)
    (Variables|Default|SetDestroyed (Variables|Default|GetDestroy))))

(event EventInteractFire
  (Variables|Default|SetDestroy true)
  (if (not (Variables|Default|GetDestroyed))
    (Variables|Default|SetActive (not (Variables|Default|GetActive)))
    (CallFunction|TriggerActive)
    (Variables|Default|SetDestroyed (Variables|Default|GetDestroy))))

(fn ConstructionScript
  (|CallParentFunction))

(fn TriggerActive
  (bind _active (Variables|Default|GetActive))
  (Rendering|SetVisibility (Variables|Default|GetCube) (Variables|Default|GetActive) false)
  (Physics|SetSimulatePhysics (Variables|Default|GetCube) (Variables|Default|GetActive))
  (Collision|SetActorEnableCollision _active)
  (Class|SceneComponent|AddWorldTransform (Variables|Default|GetCube) (Math|Transform|MakeTransform (Math|Vector|MakeVector 0.0 0.0 (select _active -5e+02 5e+02)) "0, 0, 0" "1.000000,1,1") false true) ; Move out of way for the sake of movement
)